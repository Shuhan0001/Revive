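; BP_TestCube is a talkable NPC pawn, apparently a dog, that follows the player once its dialogue finishes.
; A box overlap fades the interact-tip widget and toggles input.
; StartTalkingWithDog types successive NPC StoryLines into a timed speech bubble, then sets IsFollowing, enabling per-tick AIMoveTo and a fixed follow-up line.
; Player-speaker display is disconnected, and that branch checks only IsPlayerSpeaking's first entry without advancing the line.
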(event `self.ReceiveTick`
  (params (DeltaSeconds :type "Float (single-precision)"))
  (if (`self.IsFollowing`)
    (`|AIMoveTo` self (0.0 0.0 0.0) (`GameplayStatics.GetPlayerCharacter` 0) 100.0)))

(event `self.ReceiveBeginPlay`
  (`|ExecutionSequence`
    (:`then_0`
      (bind _aswbp_interact_tip (cast `/Game/Lib_items/BluePrint/WBP_InteractTip` (`WidgetComponent.GetUserWidgetObject` (`self.Widget`))))
      (set `self.MyUI_Ref` _aswbp_interact_tip))))

(event `self.Box.OnComponentBeginOverlap`
  (params (OverlappedComponent :type "PrimitiveComponent Object Reference") (OtherActor :type "Actor Object Reference") (OtherComp :type "PrimitiveComponent Object Reference") (OtherBodyIndex :type Integer) (bFromSweep :type Boolean) (SweepResult :type "HitResult Structure (by ref)"))
  (bind _myui_ref (`self.MyUI_Ref`))
  (`UserWidget.PlayAnimation` _myui_ref (`/Game/Lib_items/BluePrint/WBP_InteractTip.FadeAni` _myui_ref) 0.0 1 "Forward" 1.0 false)
  (`self.EnableInput` (`GameplayStatics.GetPlayerController` 0)))

(event `self.Box.OnComponentEndOverlap`
  (params (OverlappedComponent :type "PrimitiveComponent Object Reference") (OtherActor :type "Actor Object Reference") (OtherComp :type "PrimitiveComponent Object Reference") (OtherBodyIndex :type Integer))
  (bind _myui_ref (`self.MyUI_Ref`))
  (`UserWidget.PlayAnimation` _myui_ref (`/Game/Lib_items/BluePrint/WBP_InteractTip.FadeAni` _myui_ref) 0.0 1 "Reverse" 1.0 false)
  (`self.DisableInput` (`GameplayStatics.GetPlayerController` 0)))

(event `Start Talking With Dog`
  (bind _currentline (`self.CurrentLine`))
  (bind _dialogbubble (`self.DialogBubble`))
  (if (`self.IsFollowing`)
    (bind _aswbp_dialogue (cast `/Game/Lib_items/BluePrint/WBP_Dialogue` (`WidgetComponent.GetUserWidgetObject` (`self.DialogBubble`))))
    (`/Game/Lib_items/BluePrint/WBP_Dialogue.StartTypewriter` _aswbp_dialogue "Are we there yet?")
    (`SceneComponent.SetVisibility` _dialogbubble true false :!label _label)
    (set `self.CurrentLine` (+ (`self.CurrentLine`) 1))
    (`KismetSystemLibrary.RetriggerableDelay` 10.0)
    (`SceneComponent.SetVisibility` _dialogbubble false false)
    (else
      (`KismetSystemLibrary.PrintString` "Hello")
      (if (< _currentline (`KismetArrayLibrary.Array_Length` (`self.StoryLines`)))
        (if (`|GetArrayItem` (`self.IsPlayerSpeaking`))
          (bind _asbp_main_role (cast `/Game/BP_MainRole` (`GameplayStatics.GetPlayerCharacter` 0)))
          (else
            (bind _aswbp_dialogue_2 (cast `/Game/Lib_items/BluePrint/WBP_Dialogue` (`WidgetComponent.GetUserWidgetObject` (`self.DialogBubble`))))
            (`/Game/Lib_items/BluePrint/WBP_Dialogue.StartTypewriter` _aswbp_dialogue_2 (`KismetTextLibrary.Conv_TextToString` (`KismetTextLibrary.Conv_StringToText` (`|GetArrayItem` (`self.StoryLines`) _currentline))))
            (goto _label)))
        (else
          (`SceneComponent.SetVisibility` (`self.DialogBubble`) false false)
          (set `self.CurrentLine` 0)
          (set `self.IsFollowing` true))))))

(fn `UserConstructionScript`)