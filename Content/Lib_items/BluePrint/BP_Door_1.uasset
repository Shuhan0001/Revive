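; BP_Door_1 is an interactable hinged door that the player opens and closes with the E key.
; Overlapping InteractZone fades in a WBP_InteractTip widget and enables input on the door; leaving reverses the fade and disables input.
; Each E press alternates through a FlipFlop between playing and reversing the DoorSwing timeline, which drives the Hinge component's relative yaw.
; Overlaps are not filtered by actor, and player controller 0 always receives the input toggle.
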(event `self.InteractZone.OnComponentBeginOverlap`
  (params (OverlappedComponent :type "PrimitiveComponent Object Reference") (OtherActor :type "Actor Object Reference") (OtherComp :type "PrimitiveComponent Object Reference") (OtherBodyIndex :type Integer) (bFromSweep :type Boolean) (SweepResult :type "HitResult Structure (by ref)"))
  (bind _my_ui_ref (`self.My UI Ref`))
  (`UserWidget.PlayAnimation` _my_ui_ref (`/Game/Lib_items/BluePrint/WBP_InteractTip.FadeAni` _my_ui_ref) 0.0 1 "Forward" 1.0 false)
  (`self.EnableInput` (`GameplayStatics.GetPlayerController` 0)))

(event `self.ReceiveBeginPlay`
  (bind _aswbp_interact_tip (cast `/Game/Lib_items/BluePrint/WBP_InteractTip` (`WidgetComponent.GetUserWidgetObject` (`self.Widget`))))
  (set `self.My UI Ref` _aswbp_interact_tip))

(event `self.InteractZone.OnComponentEndOverlap`
  (params (OverlappedComponent :type "PrimitiveComponent Object Reference") (OtherActor :type "Actor Object Reference") (OtherComp :type "PrimitiveComponent Object Reference") (OtherBodyIndex :type Integer))
  (bind _my_ui_ref (`self.My UI Ref`))
  (`UserWidget.PlayAnimation` _my_ui_ref (`/Game/Lib_items/BluePrint/WBP_InteractTip.FadeAni` _my_ui_ref) 0.0 1 "Reverse" 1.0 false)
  (`self.DisableInput` (`GameplayStatics.GetPlayerController` 0)))

(event `Key|E`
  (params (Key :type "Key Structure"))
  (:`Pressed`
    (`/Engine/EditorBlueprintResources/StandardMacros.FlipFlop`
      (:`A`
        (bind (_direction _angle) (`Timeline|Door Swing` :!label _label)
          (:`Update`
            (`SceneComponent.K2_SetRelativeRotation` (`self.Hinge`) (`KismetMathLibrary.MakeRotator` 0.0 0.0 _angle) false false))))
      (:`B`
        (goto _label :!via `Reverse`)))))

(fn `UserConstructionScript`)