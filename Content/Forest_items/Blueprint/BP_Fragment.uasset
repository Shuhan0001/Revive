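; BP_Fragment is a collectible forest item that raises the CollectedFragments count on BP_MainRole when the player character touches it.
; A timeline started on BeginPlay drives the paper sprite's relative Z for a floating motion.
; On sphere overlap it increments the count, plays a pickup sound at world origin, then hides itself and disables collision instead of being destroyed.
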(event `self.ReceiveBeginPlay`
  (bind (_direction _floatz) (`Timeline|TL_Floating`)
    (:`Update`
      (`SceneComponent.K2_SetRelativeLocation` (`self.PaperSprite`) (`KismetMathLibrary.MakeVector` 0.0 0.0 _floatz) false false))))

(event `self.Sphere.OnComponentBeginOverlap`
  (params (OverlappedComponent :type "PrimitiveComponent Object Reference") (OtherActor :type "Actor Object Reference") (OtherComp :type "PrimitiveComponent Object Reference") (OtherBodyIndex :type Integer) (bFromSweep :type Boolean) (SweepResult :type "HitResult Structure (by ref)"))
  (bind _asbp_main_role (cast `/Game/BP_MainRole` OtherActor))
  (set `/Game/BP_MainRole.CollectedFragments` (+ (`/Game/BP_MainRole.CollectedFragments` _asbp_main_role) 1) _asbp_main_role)
  (`GameplayStatics.PlaySoundAtLocation` "/Game/Characters/SoundPack/wav__HD_/JDSherbert_-_Pixel_UI_SFX_Pack_-_Cancel_1__Square_.JDSherbert_-_Pixel_UI_SFX_Pack_-_Cancel_1__Square_" (0.0 0.0 0.0) (struct) 1.0 1.0 0.0 null null null null)
  (`self.SetActorHiddenInGame` true)
  (`self.SetActorEnableCollision` false))

(fn `UserConstructionScript`)