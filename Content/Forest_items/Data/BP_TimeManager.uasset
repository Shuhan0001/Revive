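; BP_TimeManager controls the level's time of day, switching sun and fog between presets in LightingSettings.
; BeginPlay applies a random preset and caches "MagicSpot"-tagged spotlights, which are otherwise unused here.
; DayChange cycles through three presets, using a timeline to lerp sun pitch, sun color and fog color.
; Every timeline update also unhides all BP_Fragment actors and enables their collision; OnSteleRepaired is an empty stub.
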(event `self.ReceiveBeginPlay`
  (bind _sunlight (`self.SunLight`))
  (bind _outactors (`GameplayStatics.GetAllActorsOfClassWithTag` "/Script/Engine.SpotLight" "MagicSpot"))
  (set `self.SpotLightArray` _outactors)
  (bind _output_get (set `self.CurrentIndex` (`KismetMathLibrary.RandomIntegerInRange` 0 (- (`KismetArrayLibrary.Array_Length` (`self.LightingSettings`)) 1))))
  (bind (_sunpitch _suncolor _fogcolor) (break `/Game/Forest_items/Data/S_LightingConfig` (`|GetArrayItem` (`self.LightingSettings`) _output_get)))
  (`self.K2_SetActorRotation` _sunlight (`KismetMathLibrary.MakeRotator` 0.0 _sunpitch) false)
  (`LightComponent.SetLightColor` (`Light.LightComponent` _sunlight) _suncolor true)
  (`ExponentialHeightFogComponent.SetFogInscatteringColor` (`ExponentialHeightFog.Component` (`self.WeatherFog`)) _fogcolor))

(event `OnSteleRepaired`)

(event `DayChange`
  (bind (_sunpitch _suncolor _fogcolor) (break `/Game/Forest_items/Data/S_LightingConfig` (`self.StartLightData`)))
  (bind (_sunpitch_2 _suncolor_2 _fogcolor_2) (break `/Game/Forest_items/Data/S_LightingConfig` (`self.TargetLightData`)))
  (`KismetSystemLibrary.PrintString` "1")
  (set `self.StartLightData` (`|GetArrayItem` (`self.LightingSettings`) (`self.CurrentIndex`)))
  (set `self.CurrentIndex` (mod (+ (`self.CurrentIndex`) 1) 3))
  (set `self.TargetLightData` (`|GetArrayItem` (`self.LightingSettings`) (`self.CurrentIndex`)))
  (bind (_direction _alpha) (`Timeline|TimeTransition` :!via `PlayFromStart`)
    (:`Update`
      (`self.K2_SetActorRotation` (`self.SunLight`) (`KismetMathLibrary.MakeRotator` 0.0 (`KismetMathLibrary.Lerp` _sunpitch _sunpitch_2 _alpha)) false)
      (`LightComponent.SetLightColor` (`Light.LightComponent` (`self.SunLight`)) (`KismetMathLibrary.LinearColorLerp` _suncolor _suncolor_2 _alpha) true)
      (`ExponentialHeightFogComponent.SetFogInscatteringColor` (`ExponentialHeightFog.Component` (`self.WeatherFog`)) (`KismetMathLibrary.LinearColorLerp` _fogcolor _fogcolor_2 _alpha))
      (bind _outactors (`GameplayStatics.GetAllActorsOfClass` "/Game/Forest_items/Blueprint/BP_Fragment.BP_Fragment_C"))
      (for _array_element _outactors
        (`self.SetActorHiddenInGame` _array_element false)
        (`self.SetActorEnableCollision` _array_element true)))))

(fn `UserConstructionScript`)