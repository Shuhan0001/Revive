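; BP_Mashmellow is a campfire marshmallow pickup that the player eats with the E key, also acting as a save point.
; A box overlap with BP_MainRole enables input on the actor, and leaving disables it.
; Pressing E swaps the Paper2D sprite to empty and writes the player's transform to a new BP_SaveGame in a fixed slot.
; A DoOnce limits the eating sound to the first press, though saving repeats.
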(event `self.ReceiveBeginPlay`)

(event `Key|E` :consume false
  (params (Key :type "Key Structure"))
  (:`Pressed`
    (`PaperSpriteComponent.SetSprite` (`self.PaperSprite`) (`self.Sprite_Empty`))
    (bind _returnvalue (`GameplayStatics.CreateSaveGameObject` "/Game/Forest_items/Blueprint/BP_SaveGame.BP_SaveGame_C"))
    (set `/Game/Forest_items/Blueprint/BP_SaveGame.PlayerSavedTransform` (`self.GetTransform` (`GameplayStatics.GetPlayerCharacter` 0)) _returnvalue)
    (`GameplayStatics.SaveGameToSlot` _returnvalue "save1")
    (`/Engine/EditorBlueprintResources/StandardMacros.DoOnce` false
      (:`Completed`
        (`GameplayStatics.PlaySound2D` "/Game/Characters/SoundPack/wav__HD_/Eat_Cue.Eat_Cue" 1.0 1.0 0.0 null null)))))

(event `self.Box.OnComponentBeginOverlap`
  (params (OverlappedComponent :type "PrimitiveComponent Object Reference") (OtherActor :type "Actor Object Reference") (OtherComp :type "PrimitiveComponent Object Reference") (OtherBodyIndex :type Integer) (bFromSweep :type Boolean) (SweepResult :type "HitResult Structure (by ref)"))
  (cast `/Game/BP_MainRole` OtherActor)
  (`self.EnableInput` (`GameplayStatics.GetPlayerController` 0)))

(event `self.Box.OnComponentEndOverlap`
  (params (OverlappedComponent :type "PrimitiveComponent Object Reference") (OtherActor :type "Actor Object Reference") (OtherComp :type "PrimitiveComponent Object Reference") (OtherBodyIndex :type Integer))
  (cast `/Game/BP_MainRole` OtherActor)
  (`self.DisableInput` (`GameplayStatics.GetPlayerController` 0)))

(fn `UserConstructionScript`)